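; Sliding double door that the player unlocks through a hacking minigame.
; The trigger box shows a prompt widget and arms interaction for the first-person character; pressing E then fades the camera and possesses the Bp_MiniGame actor found in the level.
; OpenDoor, meant to follow a successful hack, destroys the widget, waits briefly, then uses a timeline to lerp both panels from their starting relative positions to fixed open offsets.
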(event OnComponentBeginOverlap(Box)
  (params (OverlappedComponent :type Primitive%20Component%20Object%20Reference) (OtherActor :type Actor%20Object%20Reference) (OtherComp :type Primitive%20Component%20Object%20Reference) (OtherBodyIndex :type Integer) (bFromSweep :type Boolean) (SweepResult :type Hit%20Result%20Structure%20%28by%20ref%29))
  ;[1 1 1] Overlap Event logic when the player goes close to the door, revealing the hacking symbol
  (Utilities|Casting|CastToBP_FirstPersonCharacter OtherActor)
  (Variables|Default|SetInteract true)
  (Input|EnableInput (Game|GetPlayerController 0))
  (Rendering|SetVisibility (Variables|Default|GetWidget) true false))

(event OnComponentEndOverlap(Box)
  (params (OverlappedComponent :type Primitive%20Component%20Object%20Reference) (OtherActor :type Actor%20Object%20Reference) (OtherComp :type Primitive%20Component%20Object%20Reference) (OtherBodyIndex :type Integer))
  ;[1 1 1] Overlap Event logic when the player goes close to the door, revealing the hacking symbol
  (Utilities|Casting|CastToBP_FirstPersonCharacter OtherActor)
  (Variables|Default|SetInteract false)
  (Rendering|SetVisibility (Variables|Default|GetWidget) false false))

(event Custom|OpenDoor
  ;[1 1 1] Involves with logic of door openning sequence using timeline after a successful attempt with hacking.
  (Components|DestroyComponent (Variables|Default|GetWidget))
  (Utilities|FlowControl|Delay 1.0)
  (bind _alpha (Timeline|Timeline PlayFromStart)
    (:Update
      (Transformation|SetRelativeLocation (Variables|Default|GetLeft) (Math|Vector|Lerp(Vector) (Variables|Default|GetRelative%20Location%20Left) "-63.000000,0.000000,0.000000" _alpha) false false)
      (Transformation|SetRelativeLocation (Variables|Default|GetRight) (Math|Vector|Lerp(Vector) (Variables|Default|GetRelative%20Location%20Right) "63.000000,0.000000,0.000000" _alpha) false false))))

(event EventBeginPlay
  ;[1 1 1] Initializing door variables at the start of the game
  (Variables|Default|SetRelative%20Location%20Left (Variables|/Script/Engine.SceneComponent|GetRelativeLocation (Variables|Default|GetLeft)))
  (Variables|Default|SetRelative%20Location%20Right (Variables|/Script/Engine.SceneComponent|GetRelativeLocation (Variables|Default|GetRight))))

(event Input|KeyboardEvents|E
  (params (Key :type Key%20Structure :default "None"))
  ;[1 1 1] Interacting with door logic so that it transitions into the hacking circuit scene.
  (:Pressed
    (if (Variables|Default|GetInteract)
      (CameraFades|StartCameraFade :self (Game|GetPlayerCameraManager 0) :FromAlpha 1.0 :Duration 1.0)
      (bind _returnvalue (Actor|GetActorOfClass "/Game/Blueprints/Bp_MiniGame.Bp_MiniGame_C"))
      (Pawn|Possess (Game|GetPlayerController 0) _returnvalue))))

(fn ConstructionScript)