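; Possessable steering mini-game where arrow keys turn a continuously moving Line component, aiming to reach an End-tagged component.
; Possession starts movement after a short delay, and Tick offsets the Line along the current direction.
; Sphere overlap with End shows the win widget; any other overlap counts a fail, resets the Line and shows restart, or lost on the third.
; Each outcome pauses the game.
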(event OnComponentBeginOverlap(Sphere)
  (params (OverlappedComponent :type Primitive%20Component%20Object%20Reference) (OtherActor :type Actor%20Object%20Reference) (OtherComp :type Primitive%20Component%20Object%20Reference) (OtherBodyIndex :type Integer) (bFromSweep :type Boolean) (SweepResult :type Hit%20Result%20Structure%20%28by%20ref%29))
  ;[1 1 1] Logic for Sphere Object Collision Detection, Delay, and Position Reset
  (if (Components|ComponentHasTag OtherComp "End")
    (Utilities|FlowControl|Delay 1.0)
    (bind _returnvalue (UserInterface|CreateWidget "/Game/UI/W_Won.W_Won_C"))
    (UserInterface|Viewport|AddtoViewport _returnvalue 0)
    (Actor|SetLifeSpan 5.0)
    (Game|SetGamePaused true)
    (else
      (bind _output_get (Variables|Default|SetFail (+ (Variables|Default|GetFail) 1)))
      (if (== _output_get 3)
        (bind _returnvalue_2 (UserInterface|CreateWidget "/Game/UI/W_Lost.W_Lost_C"))
        (UserInterface|Viewport|AddtoViewport _returnvalue_2 0)
        (CallFunction|ResetMiniGame)
        (Game|SetGamePaused true)
        (else
          (bind _returnvalue_3 (UserInterface|CreateWidget "/Game/UI/W_Retstart.W_Retstart_C"))
          (UserInterface|Viewport|AddtoViewport _returnvalue_3 0)
          (CallFunction|ResetMiniGame)
          (Game|SetGamePaused true))))))

(event Custom|ResetMiniGame
  (Transformation|SetRelativeTransform (Variables|Default|GetLine) (Variables|Default|GetDefault%20Transform) false true)
  (Variables|Default|SetDirection "NewEnumerator0")
  (if (== (Variables|Default|GetFail) 3)
    (Variables|Default|SetFail 0)))

(event EventTick
  (params (DeltaSeconds :type Float%20%28single-precision%29))
  (bind _line (Variables|Default|GetLine))
  ;[1 1 1] This logic handles the movement of a sphere object, ensuring it continuously moves in one direction (until the player makes it turn any other direction).
  (if (Variables|Default|GetStart)
    (switch Utilities|FlowControl|Switch|SwitchonE_Direction (Variables|Default|GetDirection)
      (:NewEnumerator0
        (Transformation|AddLocalOffset _line "5.000000,0.000000,0.000000" false false))
      (:NewEnumerator1
        (Transformation|AddLocalOffset _line "-5.000000,0.000000,0.000000" true false))
      (:NewEnumerator2
        (Transformation|AddLocalOffset _line "0.000000,-5.000000,0.000000" true false))
      (:NewEnumerator3
        (Transformation|AddLocalOffset _line "0.000000,5.000000,0.000000" true false)))))

(event EventBeginPlay
  (Variables|Default|SetDefault%20Transform (Transformation|GetRelativeTransform (Variables|Default|GetLine)))
  (Variables|Default|SetStart false))

(event EventPossessed
  (params (NewController :type Controller%20Object%20Reference))
  (Variables|Default|SetStart false)
  (Utilities|FlowControl|Delay 1.0)
  (Variables|Default|SetStart true))

(event EventUnpossessed
  (params (OldController :type Controller%20Object%20Reference))
  (Variables|Default|SetStart false))

(event Input|KeyboardEvents|Left
  (params (Key :type Key%20Structure :default "None"))
  ;[1 1 1] Keybinds for the sphere to move in keyboard
  (:Pressed
    (Variables|Default|SetDirection "NewEnumerator3")))

(event Input|KeyboardEvents|Right
  (params (Key :type Key%20Structure :default "None"))
  ;[1 1 1] Keybinds for the sphere to move in keyboard
  (:Pressed
    (Variables|Default|SetDirection "NewEnumerator2")))

(event Input|KeyboardEvents|Up
  (params (Key :type Key%20Structure :default "None"))
  ;[1 1 1] Keybinds for the sphere to move in keyboard
  (:Pressed
    (Variables|Default|SetDirection "NewEnumerator1")))

(event Input|KeyboardEvents|Down
  (params (Key :type Key%20Structure :default "None"))
  ;[1 1 1] Keybinds for the sphere to move in keyboard
  (:Pressed
    (Variables|Default|SetDirection "NewEnumerator0")))

(fn ConstructionScript)